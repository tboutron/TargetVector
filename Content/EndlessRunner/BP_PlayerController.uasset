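; Player controller for the endless runner that builds the local player's CommonUI layout and toggles an EOS menu.
; On BeginPlay it asynchronously creates CBW_PrimaryLayout, suspending input until done, caches its game, menu and modal stacks, and pushes Common_EOSMainWidget onto the game layer stack.
; The OpenMenu input adds or removes Common_EOS on that same stack, switching mouse cursor and input mode to match.
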(event EventBeginPlay
  (|CallParentFunction)
  (if (Pawn|IsLocalPlayerController)
    (bind _userwidget (|WidgetAsync "/Game/UI/CommonUI/CBW_PrimaryLayout.CBW_PrimaryLayout_C" self true)
      (:OnComplete
        (UserInterface|Viewport|AddtoViewport _userwidget 0)
        (bind _ascbw_primary_layout (Utilities|Casting|CastToCBW_PrimaryLayout _userwidget))
        (Variables|Default|SetGame%20Layer%20Stack (Variables|/Game/UI/CommonUI/CBW_PrimaryLayout.CBW_PrimaryLayout_C|GetGameLayer_Stack _ascbw_primary_layout))
        (Variables|Default|SetGame%20Menu%20Stack (Variables|/Game/UI/CommonUI/CBW_PrimaryLayout.CBW_PrimaryLayout_C|GetGameMenu_Stack _ascbw_primary_layout))
        (Variables|Default|SetMenu%20Stack (Variables|/Game/UI/CommonUI/CBW_PrimaryLayout.CBW_PrimaryLayout_C|GetMenu_Stack _ascbw_primary_layout))
        (Variables|Default|SetModal%20Queue (Variables|/Game/UI/CommonUI/CBW_PrimaryLayout.CBW_PrimaryLayout_C|GetModal_Queue _ascbw_primary_layout))
        (Class|CommonActivatableWidgetContainerBase|AddWidget (Variables|Default|GetGame%20Layer%20Stack) "/Game/EndlessRunner/Common_EOSMainWidget.Common_EOSMainWidget_C")))))

(event Input|ActionEvents|InputActionOpenMenu
  (params (Key :type Key%20Structure :default "None"))
  (bind _self self)
  (bind _self_2 self)
  (:Pressed
    (if (Pawn|IsLocalPlayerController)
      (Variables|Default|GetEOSMenu
        (:then
          (Class|CommonActivatableWidgetContainerBase|RemoveWidget (Variables|Default|GetGame%20Layer%20Stack) (Variables|Default|GetEOSMenu))
          (Variables|Default|SetEOSMenu 0)
          (Variables|/Script/Engine.PlayerController|SetbShowMouseCursor _self_2 false)
          (Input|SetInputModeGameOnly _self_2))
        (:else
          (bind _returnvalue (Class|CommonActivatableWidgetContainerBase|AddWidget (Variables|Default|GetGame%20Layer%20Stack) "/Game/EOS/Common_EOS.Common_EOS_C"))
          (bind _output_get (Variables|Default|SetEOSMenu _returnvalue))
          (Input|SetInputModeGameandUI _self _output_get "LockAlways" true)
          (Variables|/Script/Engine.PlayerController|SetbShowMouseCursor _self true))))))

(fn ConstructionScript)